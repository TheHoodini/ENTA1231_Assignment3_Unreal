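; Pinball game mode for score-based play, tracking points and remaining balls through BP_PinballGameState.
; AddScore adds incoming points to the game state's score.
; OnBallLost decrements the ball count on the game state, then spawns a new ball while any remain, or opens the MainMenu level when none are left.
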(event `self.ReceiveBeginPlay`)

(event `/Game/Blueprints/BPI_ScoreReceiver.AddScore`
  (params (AddScore :type "Float (double-precision)"))
  (bind _asbp_pinball_game_state (cast `/Game/Blueprints/BP_PinballGameState` (`GameplayStatics.GetGameState`)))
  (`/Game/Blueprints/BP_PinballGameState.SetScore` _asbp_pinball_game_state (+ (`/Game/Blueprints/BP_PinballGameState.Score` _asbp_pinball_game_state) AddScore)))

(event `self.OnBallLost`
  (bind _asbp_pinball_game_state (cast `/Game/Blueprints/BP_PinballGameState` (`GameplayStatics.GetGameState`)))
  (bind _ballsremaining (`/Game/Blueprints/BP_PinballGameState.BallsRemaining` _asbp_pinball_game_state))
  (bind _result (`/Engine/EditorBlueprintResources/StandardMacros.DecrementInt` _ballsremaining)
    (:`  `
      (`/Game/Blueprints/BP_PinballGameState.SetBalls` _asbp_pinball_game_state _result)
      (if (> _ballsremaining 0)
        (`self.SpawnBall`)
        (else
          (`GameplayStatics.OpenLevelBySoftObjectPtr` "/Game/MainMenu.MainMenu"))))))

(fn `UserConstructionScript`
  (`parent.UserConstructionScript`))