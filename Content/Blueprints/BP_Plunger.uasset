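; Pinball plunger actor that animates its mesh on Charge and Release and launches objects leaving its collision.
; Charge runs a timeline that moves the mesh between start and end positions and records ChargeTime; Release stops it and plays a second timeline.
; On end overlap, actors implementing BPI_PinballReactive receive an impulse away from the plunger, scaled by MaxForce and the last ChargeTime.
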(event `Charge`
  (bind (_direction _newtrack_0) (`Timeline|ChargeTimeline` :!via `PlayFromStart` :!label _label)
    (:`Update`
      (set `self.Charge time` _newtrack_0)
      (bind _returnvalue (`KismetMathLibrary.VLerp` (`self.StartPos`) (`self.EndPos`) _newtrack_0))
      (set `self.UpdatedPos` _returnvalue)
      (`SceneComponent.K2_SetRelativeLocation` (`self.SM_Plunger`) _returnvalue false false))))

(event `Release`
  (`|ExecutionSequence`
    (:`then_0`
      (goto _label :!via `Stop`))
    (:`then_1`
      (bind (_direction _newtrack_0) (`Timeline|Timeline_0` :!via `PlayFromStart`)
        (:`Update`
          (`SceneComponent.K2_SetRelativeLocation` (`self.SM_Plunger`) (`KismetMathLibrary.VLerp` (`self.StartPos`) (`self.EndPos`) _newtrack_0) false false))))))

(event `self.Collision.OnComponentEndOverlap`
  (params (OverlappedComponent :type "PrimitiveComponent Object Reference") (OtherActor :type "Actor Object Reference") (OtherComp :type "PrimitiveComponent Object Reference") (OtherBodyIndex :type Integer))
  (bind _asbpi_pinball_reactive (cast `/Game/Assets/BPI_PinballReactive` OtherActor))
  (`/Game/Assets/BPI_PinballReactive.PinballImpulseEvent` _asbpi_pinball_reactive (* (* (`self.MaxForce`) (`self.Charge time`)) (`KismetMathLibrary.Normal` (- (`SceneComponent.K2_GetComponentLocation` OtherComp) (`self.K2_GetActorLocation`))))))

(fn `UserConstructionScript`)