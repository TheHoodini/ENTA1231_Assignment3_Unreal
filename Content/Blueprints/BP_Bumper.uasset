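; BP_Bumper is a pinball bumper that knocks overlapping pinball-reactive actors away and awards score.
; On capsule overlap it sends a normalized outward impulse scaled by MaxForce through BPI_PinballReactive, then adds ScoreValue to the GameMode through BPI_ScoreReceiver.
; Each overlap also plays a timeline that lerps the mechanism mesh from StartPos to EndPos.
; End overlap stops the timeline and snaps the mesh back to StartPos.
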(event `self.Capsule.OnComponentBeginOverlap`
  (params (OverlappedComponent :type "PrimitiveComponent Object Reference") (OtherActor :type "Actor Object Reference") (OtherComp :type "PrimitiveComponent Object Reference") (OtherBodyIndex :type Integer) (bFromSweep :type Boolean) (SweepResult :type "HitResult Structure (by ref)"))
  (`|ExecutionSequence`
    (:`then_0`
      (bind _asbpi_pinball_reactive (cast `/Game/Assets/BPI_PinballReactive` OtherActor))
      (`/Game/Assets/BPI_PinballReactive.PinballImpulseEvent` _asbpi_pinball_reactive (* (`self.MaxForce`) (`KismetMathLibrary.Normal` (- (`SceneComponent.K2_GetComponentLocation` OtherComp) (`self.K2_GetActorLocation`)))))
      (bind _asbpi_score_receiver (cast `/Game/Blueprints/BPI_ScoreReceiver` (`GameplayStatics.GetGameMode`)))
      (`/Game/Blueprints/BPI_ScoreReceiver.AddScore` _asbpi_score_receiver (`self.ScoreValue`))
      (`KismetSystemLibrary.PrintString` "Hello"))
    (:`then_1`
      (bind (_direction _alpha) (`Timeline|Timeline` :!label _label)
        (:`Update`
          (`SceneComponent.K2_SetRelativeLocation` (`self.SM_Mechanism`) (`KismetMathLibrary.VLerp` (`self.StartPos`) (`self.EndPos`) _alpha) false false))))))

(event `self.Capsule.OnComponentEndOverlap`
  (params (OverlappedComponent :type "PrimitiveComponent Object Reference") (OtherActor :type "Actor Object Reference") (OtherComp :type "PrimitiveComponent Object Reference") (OtherBodyIndex :type Integer))
  (`|ExecutionSequence`
    (:`then_0`
      (goto _label :!via `Stop`))
    (:`then_1`
      (`SceneComponent.K2_SetRelativeLocation` (`self.SM_Mechanism`) (`self.StartPos`) false false))))

(fn `UserConstructionScript`)