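; Pinball actor that spawns BP_Ball instances at its own location through its SpawnBall function.
; On BeginPlay it registers itself as the BallSpawner on BP_PinballGameMode_Base, giving the game mode a reference to it.
; An older spawn at a randomized position is left disconnected in the event graph and never runs.
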(event `self.ReceiveBeginPlay`
  (bind _asbp_pinball_game_mode_base (cast `/Game/Blueprints/BP_PinballGameMode_Base` (`GameplayStatics.GetGameMode`)))
  (set `/Game/Blueprints/BP_PinballGameMode_Base.BallSpawner` self _asbp_pinball_game_mode_base))

(event `self.ReceiveActorBeginOverlap`
  (params (OtherActor :type "Actor Object Reference")))

(event `self.ReceiveTick`
  (params (DeltaSeconds :type "Float (single-precision)")))

(fn `SpawnBall`
  (`|SpawnActorFromClass` "/Game/Blueprints/BP_Ball.BP_Ball_C" (`KismetMathLibrary.MakeTransform` (`self.K2_GetActorLocation`)) "Undefined" "MultiplyWithRoot" null null))

(fn `UserConstructionScript`)