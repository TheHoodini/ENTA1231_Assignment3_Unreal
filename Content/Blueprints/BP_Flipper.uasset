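; BP_Flipper is a flipper actor that swings a pivot component between a rest and a flipped rotation.
; BeginPlay sets the rest rotation to zero and derives the flipped rotation as a quarter turn, with its sign chosen by the Direction enum.
; Activate and deactivate events play and reverse a timeline, whose track lerps the Pivot's relative rotation between the two.
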(event `OnActivate_Event`
  (bind (_direction _newtrack_0) (`Timeline|0-1` :!label _label)
    (:`Update`
      (`SceneComponent.K2_SetRelativeRotation` (`self.Pivot`) (`KismetMathLibrary.RLerp` (`self.FlipperRest`) (`self.FlipperFlip`) _newtrack_0) false false))))

(event `OnDeactivate_Event`
  (goto _label :!via `Reverse`))

(event `self.ReceiveBeginPlay`
  (bind _output_get (set `self.FlipperRest` (struct)))
  (set `self.FlipperFlip` (`KismetMathLibrary.ComposeRotators` _output_get (`KismetMathLibrary.SelectRotator` (struct :`Yaw` -90.0) (struct :`Yaw` 90.0) (`|EnumEquality` (`self.Direction`) "NewEnumerator0")))))

(fn `UserConstructionScript`)